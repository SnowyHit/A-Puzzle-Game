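; Data manager for a puzzle game that fetches the puzzle JSON on BeginPlay and loads an image for each piece.
; After a successful request, GetAndSetPieceImage downloads images one at a time, storing each texture by piece ID and re-calling itself with the next index.
; Once all pieces are filled, it passes them to PC_Puzzle to add to the HUD.
; A failed download is only logged, which halts the chain before the HUD receives any pieces.
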(event Custom|GetAndSetPieceImage
  (params (DownloadingPieceIndex :type Integer))
  (bind _returnvalue (Class|PuzzleDataManager|GetPieces))
  (bind _returnvalue_2 (Utilities|Array|Length _returnvalue))
  (bind _output (Utilities|Array|Get(acopy) _returnvalue DownloadingPieceIndex))
  (bind _imageurl (Utilities|Struct|BreakPuzzlePieceData _output))
  (if (> DownloadingPieceIndex -1)
    (if (== _returnvalue_2 DownloadingPieceIndex)
      (bind _aspc_puzzle (Utilities|Casting|CastToPC_Puzzle (Game|GetPlayerController 0)))
      (Default|AddPuzzlePiecestoHUD _aspc_puzzle _returnvalue)
      (elif (< DownloadingPieceIndex _returnvalue_2)
        (bind _texture (|DownloadImage _imageurl)
          (:then
            (Utilities|String|LogString (Utilities|String|Append "Starting to Download Image" _imageurl)))
          (:OnSuccess
            (Utilities|String|LogString (Utilities|String|Append "Image Downloaded From" _imageurl))
            (Class|PuzzleDataManager|FillPuzzlePieceDataImagebyID (.ID (Utilities|Struct|BreakPuzzlePieceData (Utilities|Array|Get(acopy) _returnvalue DownloadingPieceIndex))) _texture)
            (bind _result (Math|Integer|IncrementInt (Variables|Default|GetCurrentDownloadingPieceIndex))
              (:%20%20
                (CallFunction|GetandSetPieceImage _result))))
          (:OnFail
            (Utilities|String|LogString "Download Failed")))
        (else
          (Utilities|String|LogString "Given İndex is greater than the value of pieces array."))))
    (else
      (Utilities|String|LogString "The Given index is not correct."))))

(event EventBeginPlay
  (Class|PuzzleDataManager|RequestPuzzleJSON))

(event EventOnRequestCompletedBPEvent
  (params (Success :type Boolean))
  (if Success
    (Variables|Default|SetCurrentDownloadingPieceIndex 0)
    (CallFunction|GetandSetPieceImage (Variables|Default|GetCurrentDownloadingPieceIndex))))

(fn ConstructionScript)