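; Puzzle game state that bridges puzzle progress to the HUD widget and shows the submit screen when all pieces are correctly placed.
; After a one-tick delay it caches the widget from BP_PuzzleHUD, then pushes elapsed time every Tick.
; Moves and deletions call parent logic, then refresh move count and the board's unplaced pieces.
; Initial piece data is shuffled into the HUD's image grid.
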(event Custom|AddPuzzlePiecesToHUD
  (params (PuzzlePieceDatas :type Array%20of%20Puzzle%20Piece%20Data%20Structures))
  ;[1 1 1] Initial HUD Setup for first download
  (Utilities|Array|Shuffle PuzzlePieceDatas)
  (Default|SetupImageGrid (Variables|Default|GetHUDWidget) PuzzlePieceDatas))

(event Custom|UpdateHUDPieces
  ;[1 1 1] Updates HUD with pieces that placed on board
  (bind _returnvalue (Actor|GetActorOfClass "/Game/Blueprints/BP_PuzzleBoard.BP_PuzzleBoard_C"))
  (Default|CheckPiecesandUpdateUI (Variables|Default|GetHUDWidget) (Class|PuzzleBoard|GetPiecesNotonBoard _returnvalue)))

(event EventBeginPlay
  ;[1 1 1] Setting Defaults , Waiting for a tick to make it not null ref problems
  (Utilities|FlowControl|DelayUntilNextTick)
  (bind _asbp_puzzle_hud (Utilities|Casting|CastToBP_PuzzleHUD (HUD|GetHUD (Game|GetPlayerController 0))))
  (Variables|Default|SetHUDWidget (Variables|/Game/UI/BP_PuzzleHUD.BP_PuzzleHUD_C|GetHUDWidget _asbp_puzzle_hud))
  (Variables|Default|SetUpdateTime true))

(event EventTick
  (params (DeltaSeconds :type Float%20%28single-precision%29))
  (if (Variables|Default|GetUpdateTime)
    (Default|UpdateElapsedTime (Variables|Default|GetHUDWidget) (Variables|Default|GetElapsedPuzzleTime))))

(event EventMoveMade
  (|CallParentFunction)
  (Utilities|FlowControl|Sequence
    (:then_0
      (Default|UpdateMoveCount (Variables|Default|GetHUDWidget) (Variables|Default|GetMoveCount)))
    (:then_1
      (CallFunction|UpdateHUDPieces))))

(event EventPieceDeleted
  (params (CountAsMove :type Boolean))
  (|CallParentFunction CountAsMove)
  (Utilities|FlowControl|Sequence
    (:then_0
      (Default|UpdateMoveCount (Variables|Default|GetHUDWidget) (Variables|Default|GetMoveCount)))
    (:then_1
      (CallFunction|UpdateHUDPieces))))

(event EventAllPiecesatCorrectSpot
  ;[1 1 1] Win Condition
  (Default|ShowSubmitScreen (Variables|Default|GetHUDWidget) (Variables|Default|GetMoveCount) (Variables|Default|GetElapsedPuzzleTime)))

(fn ConstructionScript)