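; PC_Puzzle is a puzzle game controller that turns a finished piece drag into a piece placed on the board in the world.
; OnDragEnded line traces on Visibility from the given world position and direction to find the drop point.
; It spawns a BP_PuzzlePiece at the origin, initializes it from the dragged data and passes it to the Board to drop or replace at the impact point, without checking for a hit.
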(event Custom|OnDragEnded
  (params (DragedPiece :type Puzzle%20Piece%20Data%20Structure) (World%20Pos :type Vector) (World%20Dir :type Vector))
  (bind _outhit (Collision|LineTraceByChannel World%20Pos (+ World%20Pos (* World%20Dir 6e+03)) "TraceTypeQuery1" false 0 "None"))
  (bind _returnvalue (Game|SpawnActorfromClass "/Game/Blueprints/BP_PuzzlePiece.BP_PuzzlePiece_C" (Math|Transform|MakeTransform "0, 0, 0") "Undefined" "MultiplyWithRoot" (Game|GetPlayerController 0) 0))
  (Class|PuzzlePiece|InitializefromData _returnvalue DragedPiece)
  (Class|PuzzleBoard|DroporReplaceatWorld (Variables|Default|GetBoard) _returnvalue (.ImpactPoint (Collision|BreakHitResult _outhit))))

(event EventBeginPlay)

(event EventTick
  (params (DeltaSeconds :type Float%20%28single-precision%29)))

(fn ConstructionScript)